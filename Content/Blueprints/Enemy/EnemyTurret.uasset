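; Enemy turret that sweeps between placed target actors, then tracks and shoots the player when spotted.
; Tick runs a Searching, Found and Returning state machine, easing rotation with RInterpTo in each state.
; PawnSensing sets Found and saves the search rotation; a retriggerable delay switches to Returning once sightings stop, resuming search at that rotation.
; While Found, a forward line trace hitting the player deals damage, gated by a reload delay.
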(event OnSeePawn(PawnSensing)
  (params (Pawn :type Pawn%20Object%20Reference))
  (Utilities|Casting|CastToWraithPlayerCharacter Pawn)
  (Utilities|FlowControl|Sequence
    (:then_0
      ;[1 1 1] Set the enemy state to found and store location if just switched
      (if (Utilities|Enum|NotEqual(Enum) (Variables|Default|GetCurrState) "NewEnumerator1")
        (Variables|Default|SetCurrState "NewEnumerator1")
        (Development|PrintString "Found player")
        (Variables|Default|SetPrevSearchLocation (Transformation|GetActorRotation self))))
    (:then_1
      ;[1 1 1] Check if turret has not see player for a set time, set to searching  again
      (Utilities|FlowControl|RetriggerableDelay 0.6)
      (Development|PrintString "start returning")
      (Variables|Default|SetCurrState "NewEnumerator2"))))

(event EventBeginPlay
  (Utilities|FlowControl|Sequence
    (:then_0
      ;[1 1 1] Calculate and store the vector from the turret to each move location
      (for _array_element (Variables|Default|GetMovePositions)
        (Utilities|Array|Add (Variables|Default|GetMoveVectors) (- (Transformation|GetActorLocation _array_element) (Transformation|GetActorLocation self)))))
    (:then_1
      ;[1 1 1] Start turret at first location
      (Transformation|SetActorRotation self (Math|Conversions|RotationFromXVector (Utilities|Array|Get(acopy) (Variables|Default|GetMoveVectors)))))))

(event EventTick
  (params (DeltaSeconds :type Float%20%28single-precision%29))
  (Utilities|FlowControl|Sequence
    (:then_0
      (switch Utilities|FlowControl|Switch|SwitchonEnemyStates (Variables|Default|GetCurrState)
        (:NewEnumerator0
          (Utilities|FlowControl|Sequence
            (:then_0
              ;[1 1 1] Move turret rotation from current rotation to next search position smoothly
              (Transformation|SetActorRotation self (Math|Interpolation|RInterpTo (Math|Conversions|RotationFromXVector (Transformation|GetActorForwardVector self)) (Math|Conversions|RotationFromXVector (Utilities|Array|Get(acopy) (Variables|Default|GetMoveVectors) (Variables|Default|GetIndexOfPositionMovingTo))) DeltaSeconds (Variables|Default|GetInterpSpeedSearching))))
            (:then_1
              ;[1 1 1] If reached target move position, set next one in list to move to
              (if (Math|Rotator|Equal(Rotator) (Transformation|GetActorRotation self) (Math|Conversions|RotationFromXVector (Utilities|Array|Get(acopy) (Variables|Default|GetMoveVectors) (Variables|Default|GetIndexOfPositionMovingTo))) (Variables|Default|GetRotationErrorEquals))
                (bind _result (Math|Integer|IncrementInt (Variables|Default|GetIndexOfPositionMovingTo))
                  (:%20%20
                    (Variables|Default|SetIndexOfPositionMovingTo (Math|Integer|%(Integer) _result (Utilities|Array|Length (Variables|Default|GetMoveVectors))))))))))
        (:NewEnumerator1
          ;[1 1 1] Turret interacts with player while player still exists
          (if (Utilities|IsValid (Game|GetPlayerCharacter 0))
            (Utilities|FlowControl|Sequence
              (:then_0
                ;[1 1 1] Smoothly rotate the turret towards the player
                (Transformation|SetActorRotation self (Math|Interpolation|RInterpTo (Math|Conversions|RotationFromXVector (Transformation|GetActorForwardVector self)) (Math|Conversions|RotationFromXVector (- (Transformation|GetActorLocation (Game|GetPlayerCharacter 0)) (Transformation|GetActorLocation self))) (Utilities|Time|GetWorldDeltaSeconds) (Variables|Default|GetInterpSpeedFound))))
              (:then_1
                ;[1 1 1] Cast line trace, shooting at player when looking directly at player, shooting then reloading
                (bind (_startloc _endloc) (CallFunction|GetStartEndOfTrace))
                (bind _outhit (Collision|LineTraceByChannel _startloc _endloc "TraceTypeQuery1" false 0 "None"))
                (Utilities|Casting|CastToWraithPlayerCharacter (.HitActor (Collision|BreakHitResult _outhit)))
                (if (not (Variables|Default|GetIsReloading))
                  (Utilities|FlowControl|Sequence
                    (:then_0
                      (bind _aswraith_player_character (Utilities|Casting|CastToWraithPlayerCharacter (Game|Player|GetPlayerPawn 0)))
                      (Default|TakeDamage _aswraith_player_character (Variables|Default|GetDamagePerShot)))
                    (:then_1
                      (Variables|Default|SetIsReloading true))
                    (:then_2
                      (Utilities|FlowControl|Delay (Variables|Default|GetTimeBetweenShots))
                      (Variables|Default|SetIsReloading false))))))))
        (:NewEnumerator2
          (Utilities|FlowControl|Sequence
            (:then_0
              ;[1 1 1] Returning back to last searching location
              (Transformation|SetActorRotation self (Math|Interpolation|RInterpTo (Transformation|GetActorRotation self) (Variables|Default|GetPrevSearchLocation) DeltaSeconds (Variables|Default|GetInterpSpeedReturning))))
            (:then_1
              ;[1 1 1] If reached prev searching location again, begin searching
              (if (Math|Rotator|Equal(Rotator) (Math|Conversions|RotationFromXVector (Transformation|GetActorForwardVector self)) (Variables|Default|GetPrevSearchLocation) (Variables|Default|GetRotationErrorEquals))
                (Development|PrintString "Start searching")
                (Variables|Default|SetCurrState "NewEnumerator0")))))))
    (:then_1
      ;[1 1 1] Debug draw for testing
      (bind (_startloc_2 _endloc_2) (CallFunction|GetStartEndOfTrace))
      (Rendering|Debug|DrawDebugLine :LineStart _startloc_2 :LineEnd _endloc_2 :Thickness 5.0))))

(fn ConstructionScript)

(fn GetStartEndOfTrace
  (return (Transformation|GetActorLocation self) (+ (* (Transformation|GetActorForwardVector self) 1e+04) (Transformation|GetActorLocation self))))