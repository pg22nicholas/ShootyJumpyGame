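; BP_GunBase is a gun Blueprint that manages magazine and reserve ammo for shooting and reloading.
; BeginPlay fills the magazine from reserve ammo, and AddAmmo increases that reserve.
; TryShoot and TryReload check ammo and state before calling Shoot or Reload, returning whether they succeeded.
; Shoot and Reload update ammo immediately and set IsShooting or IsReloading, which nothing here clears; Shoot also plays a 2D sound.
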(event EventBeginPlay
  (bind _output_get (Variables|Default|SetCurrBulletsInMagazine (Math|Integer|Min(Integer) (Variables|Default|GetAmmoOutsideMag) (Variables|Default|GetMagazineSize))))
  (Variables|Default|SetAmmoOutsideMag (- (Variables|Default|GetAmmoOutsideMag) _output_get)))

(fn ConstructionScript)

(fn TryShoot
  (if (Math|Boolean|ANDBoolean (> (Variables|Default|GetCurrBulletsInMagazine) 0) (not (Variables|Default|GetIsShooting)) (not (Variables|Default|GetIsReloading)))
    (CallFunction|Shoot)
    (return true)
    (else
      (return false))))

(fn Shoot
  (Math|Integer|DecrementInt (Variables|Default|GetCurrBulletsInMagazine)
    (:%20%20
      (Variables|Default|SetIsShooting true)
      (Audio|PlaySound2D "/Game/StarterContent/Audio/Explosion01.Explosion01" 1.0 1.0 0.0 0 0))))

(fn AddAmmo
  (params (AmmoAmount :type Integer))
  ;[1 1 1] Add ammo to overall ammo count
  (Variables|Default|SetAmmoOutsideMag (+ (Variables|Default|GetAmmoOutsideMag) AmmoAmount)))

(fn Reload
  (Utilities|FlowControl|Sequence
    (:then_0
      ;[1 1 1] Calculate number of bullets to reload into magazine
      (Variables|Default|SetAmountBulletsToLoadInMag (Math|Integer|Min(Integer) (- (Variables|Default|GetMagazineSize) (Variables|Default|GetCurrBulletsInMagazine)) (Variables|Default|GetAmmoOutsideMag))))
    (:then_1
      ;[1 1 1] Reload bullets into magazine
      (Variables|Default|SetCurrBulletsInMagazine (+ (Variables|Default|GetAmountBulletsToLoadInMag) (Variables|Default|GetCurrBulletsInMagazine))))
    (:then_2
      ;[1 1 1] Reduce amount of bullets outside magazine by amount reloaded
      (Variables|Default|SetAmmoOutsideMag (- (Variables|Default|GetAmmoOutsideMag) (Variables|Default|GetAmountBulletsToLoadInMag))))
    (:then_3
      (Variables|Default|SetIsReloading true))))

(fn TryReload
  (if (Math|Boolean|ANDBoolean (not (Variables|Default|GetIsShooting)) (not (Variables|Default|GetIsReloading)) (> (Variables|Default|GetAmmoOutsideMag) 0) (!= (Variables|Default|GetMagazineSize) (Variables|Default|GetCurrBulletsInMagazine)))
    (CallFunction|Reload)
    (return true)
    (else
      (return false))))