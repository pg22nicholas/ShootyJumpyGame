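; GunBase is a weapon Blueprint that tracks magazine bullets and overall ammo for a gun.
; BeginPlay fills the magazine up to its size, capped by the ammo count, and AddAmmo raises only the overall count.
; TryShoot gates Shoot on remaining bullets and the IsShooting flag, returning whether it fired.
; Shoot only decrements the magazine and sets IsShooting, with no reset, reload or projectile logic in this Blueprint.
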(event EventBeginPlay
  (Variables|Default|SetCurrBulletsInMagazine (Math|Integer|Min(Integer) (Variables|Default|GetMagazineSize) (Variables|Default|GetAmmoCount))))

(fn ConstructionScript)

(fn TryShoot
  (if (and (> (Variables|Default|GetCurrBulletsInMagazine) 0) (not (Variables|Default|GetIsShooting)))
    (CallFunction|Shoot)
    (return true)
    (else
      (return false))))

(fn Shoot
  (Math|Integer|DecrementInt (Variables|Default|GetCurrBulletsInMagazine)
    (:%20%20
      (Variables|Default|SetIsShooting true))))

(fn AddAmmo
  (params (AmmoAmount :type Integer))
  ;[1 1 1] Add ammo to overall ammo count
  (Variables|Default|SetAmmoCount (+ (Variables|Default|GetAmmoCount) AmmoAmount)))