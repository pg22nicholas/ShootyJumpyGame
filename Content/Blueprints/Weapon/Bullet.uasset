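; Bullet pawn that the player possesses in flight and can use to teleport the player character to its position.
; On BeginPlay it launches the Bullet component with a forward impulse, stores the player character, possesses itself and aligns the spring arm to the firing direction.
; Turn and LookUp axes drive controller yaw and pitch.
; Pressing E moves the stored character to the bullet's location, repossesses it and destroys the bullet.
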(event EventBeginPlay
  ;[1 0 0.9531] Launch Bullet and possess it
  (Physics|AddImpulse (Variables|Default|GetBullet) (* (Math|Vector|GetForwardVector (Transformation|GetActorRotation)) 1e+04) "None" false)
  (Utilities|FlowControl|Sequence
    (:then_0
      (Variables|Default|SetStoredDefaultCharacter (Game|GetPlayerCharacter 0)))
    (:then_1
      (Pawn|Possess (Game|GetPlayerController 0) self))
    (:then_2
      (Transformation|SetRelativeRotation (Variables|Default|GetSpringArm) (Math|Conversions|RotationFromXVector (Math|Vector|GetForwardVector (Transformation|GetActorRotation))) false false))))

(event Input|AxisEvents|InputAxisLookUp
  (params (AxisValue :type Float%20%28single-precision%29))
  (Pawn|Input|AddControllerPitchInput AxisValue))

(event Input|AxisEvents|InputAxisTurn
  (params (AxisValue :type Float%20%28single-precision%29))
  (Pawn|Input|AddControllerYawInput AxisValue))

(event Input|KeyboardEvents|E
  (params (Key :type Key%20Structure :default "None"))
  ;[1 1 1] Possess back to WraithPlayer at curent location of bullet
  (:Pressed
    (Transformation|SetActorLocation (Variables|Default|GetStoredDefaultCharacter) (Transformation|GetWorldLocation (Variables|Default|GetBullet)) false false)
    (Pawn|Possess (Game|GetPlayerController 0) (Variables|Default|GetStoredDefaultCharacter))
    (Actor|DestroyActor)))

(fn ConstructionScript)